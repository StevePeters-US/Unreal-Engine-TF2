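; BP_RenderTextureReader is a Blueprint that samples a render target value at the screen center every frame.
; Tick calls UpdateBuffer, then GetRenderTargetValue at half the viewport size, both defined outside this graph.
; A disconnected debug print would show the sampled color's channels as text tinted by that color, so the value is currently unused here.
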(event `self.ReceiveTick`
  (params (DeltaSeconds :type "Float (single-precision)"))
  (bind (_x _y) (`KismetMathLibrary.BreakVector2D` (/ (`WidgetLayoutLibrary.GetViewportSize`) 2.0)))
  (`self.UpdateBuffer`)
  (bind _returnvalue (`self.GetRenderTargetValue` _x _y)))

(fn `UserConstructionScript`)